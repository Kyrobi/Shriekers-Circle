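; Reverse vending machine actor that reacts when it receives a required item.
; Its ReceivedRequiredItem event instantly moves the scene root 100 units up in world Z, without sweep, on every call.
; The item check and the caller are not in this graph, and the default BeginPlay, overlap and Tick events are disabled.
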(event `self.receivedRequiredItem`
  (bind _defaultsceneroot (`self.DefaultSceneRoot`))
  (`SceneComponent.K2_SetWorldLocation` _defaultsceneroot (+ (`SceneComponent.K2_GetComponentLocation` _defaultsceneroot) (0.0 0.0 100.0)) false false))

(fn `UserConstructionScript`
  (`parent.UserConstructionScript`))