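; Dialogue character that can turn into a monster through conversation, built on a parent class's dialogue calls and BeginPlay.
; The construction script defines two option sets pairing text with codes, which CodeTrigger switches on to show options, jump or end dialogue.
; The "Monster" option's code spawns a Monster AI pawn at the actor's transform and destroys the actor.
; Greeting, jump and default branches also set Code to the monster value.
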(event `self.ReceiveBeginPlay`
  (`parent.ReceiveBeginPlay`))

(event `self.codeTrigger`
  (params (code :type Integer))
  (bind _dialogue (`self.dialogue`))
  (bind _output (`|GetArrayItem` _dialogue))
  (switch `int` code
    (:`Default`
      (`self.chooseDialogue` _output)
      (`KismetSystemLibrary.PrintString` (`self.Student`))
      (set `self.code` 3 :!label _label))
    (:`0`
      (`self.chooseDialogue` (`|GetArrayItem` _dialogue 1))
      (goto _label))
    (:`1`
      (`self.chooseDialogue` _output)
      (`self.Jump`)
      (goto _label))
    (:`2`
      (`self.endDialogue`))
    (:`3`
      (`self.chooseDialogue` (struct))
      (`self.SpawnMonster`))))

(event `SpawnMonster`
  (`AIBlueprintHelperLibrary.SpawnAIFromClass` "/Game/Blueprints/AI/Monster.Monster_C" null (`self.K2_GetActorLocation`) (`self.K2_GetActorRotation`) false null)
  (`self.K2_DestroyActor`))

(fn `UserConstructionScript`
  (set `self.dialogue` (`|MakeArray` (make `/Game/Blueprints/ST_Dialogue` (`|MakeArray` (make `/Game/Blueprints/ST_DialogueOption` "hi i'm the main character") (make `/Game/Blueprints/ST_DialogueOption` "can you jump?" 1) (make `/Game/Blueprints/ST_DialogueOption` "bye" 2) :!type "/Game/Blueprints/ST_DialogueOption Structure")) (make `/Game/Blueprints/ST_Dialogue` (`|MakeArray` (make `/Game/Blueprints/ST_DialogueOption` "Monster" 3) :!type "/Game/Blueprints/ST_DialogueOption Structure")) :!type "/Game/Blueprints/ST_Dialogue Structure")))