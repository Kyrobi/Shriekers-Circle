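; BP_InteractObject is an interactable object base that can require an item from the player's inventory.
; consumePlayerItem searches the inventory box's child widgets through PickupItem_Interface for the RequiredObject class, consumes one from the first matching stack, then fires receivedRequiredItem.
; With no required class set, it fires that event immediately.
; receivedRequiredItem and objectCodeTrigger are empty hooks here.
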(event `objectCodeTrigger`
  (params (code :type Integer)))

(event `consumePlayerItem`
  (params (playerInventory :type "/Game/Inventory/W_Inventory Object Reference"))
  (if (`KismetSystemLibrary.IsValidClass` (`self.requiredObject`))
    (for _array_element (`PanelWidget.GetAllChildren` (`/Game/Inventory/W_Inventory.InventoryBox` playerInventory))
      (bind _aspickup_item_interface (cast `/Game/Inventory/PickupItem_Interface` _array_element))
      (bind (_itemclass _currentstackamount) (`/Game/Inventory/PickupItem_Interface.GetPickupItemData` _aspickup_item_interface))
      (if (== _itemclass (`self.requiredObject`))
        (if (>= _currentstackamount 1)
          (`/Game/Inventory/PickupItem_Interface.ConsumeItems` _aspickup_item_interface 1)
          (`self.receivedRequiredItem`)
          (break)
          (else
            (break)))))
    (else
      (`self.receivedRequiredItem`))))

(event `receivedRequiredItem`)

(fn `UserConstructionScript`)