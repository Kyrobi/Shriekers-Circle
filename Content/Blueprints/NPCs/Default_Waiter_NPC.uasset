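; Default waiter NPC that idly looks around, watches the player and runs a short branching donation-request dialogue.
; A random target yaw refreshes periodically, and a self-calling next-tick loop turns toward it while no player is tracked.
; Pawn sensing snaps it to face the player, with a retriggerable delay resuming idle turning once sightings stop.
; Reply codes select dialogue from construction-script options, or end it and walk the NPC back to its starting position.
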(event `newRotation`
  (set `self.targetView` (`KismetMathLibrary.RandomRotator` false))
  (`KismetSystemLibrary.Delay` 5.0)
  (`self.newRotation`))

(event `self.ReceiveTick`
  (params (DeltaSeconds :type "Float (single-precision)"))
  (`parent.ReceiveTick` DeltaSeconds))

(event `self.ReceiveBeginPlay`
  (`parent.ReceiveBeginPlay`)
  (`self.newRotation`)
  (`self.RandomTurn`))

(event `self.PawnSensing.OnSeePawn`
  (params (Pawn :type "Pawn Object Reference"))
  (`|ExecutionSequence`
    (:`then_0`
      (if (`KismetSystemLibrary.IsValid` (`self.MainCharacter`))
        (`self.K2_SetActorRotation` (`KismetMathLibrary.FindLookAtRotation` (`SceneComponent.K2_GetComponentLocation` (`self.CapsuleComponent`)) (`SceneComponent.K2_GetComponentLocation` (`Actor.RootComponent` (`self.MainCharacter`)))) :!label _label)
        (else
          (bind _asbp_fp_character (cast `/Game/Blueprints/BP_FP_Character` Pawn)
            (:`then`
              (set `self.MainCharacter` _asbp_fp_character)
              (goto _label))
            (:`CastFailed`
              (set `self.MainCharacter` null))))))
    (:`then_1`
      (`KismetSystemLibrary.RetriggerableDelay` 0.5)
      (set `self.MainCharacter` null)
      (`self.RandomTurn`))))

(event `RandomTurn`
  (bind (_returnvalue_roll _returnvalue_pitch _returnvalue_yaw) (`KismetMathLibrary.BreakRotator` (`KismetMathLibrary.RInterpTo_Constant` (`self.K2_GetActorRotation`) (`self.targetView`) 0.2 5.0)))
  (if (not (`KismetSystemLibrary.IsValid` (`self.MainCharacter`)))
    (`self.K2_SetActorRotation` (`KismetMathLibrary.MakeRotator` 0.0 0.0 _returnvalue_yaw))
    (`KismetSystemLibrary.DelayUntilNextTick`)
    (`self.RandomTurn`)))

(event `self.codeTrigger`
  (params (code :type Integer))
  (switch `int` code
    (:`Default`
      (`self.chooseDialogue` (`|GetArrayItem` (`self.dialogue`)) "Hey! Do you have $5 to donate to less fortunate students?"))
    (:`0`
      (`self.endDialogue`)
      (`self.ReturnToPost`))
    (:`1`
      (`self.chooseDialogue` (`|GetArrayItem` (`self.dialogue`) 1) "Even if I told you they were burning alive under Strickland Hall?"))))

(event `ReturnToPost`
  (`|AIMoveTo` self (`self.Starting Position`) null
    (:`OnSuccess`
      (`self.RandomTurn`))))

(fn `UserConstructionScript`
  (`parent.UserConstructionScript`)
  (set `self.dialogue` (`|MakeArray` (make `/Game/Blueprints/ST_Dialogue` (`|MakeArray` (make `/Game/Blueprints/ST_DialogueOption` "Yes") (make `/Game/Blueprints/ST_DialogueOption` "No" 1) :!type "/Game/Blueprints/ST_DialogueOption Structure")) (make `/Game/Blueprints/ST_Dialogue` (`|MakeArray` (make `/Game/Blueprints/ST_DialogueOption` "Uhh I don't really want to, sorry") :!type "/Game/Blueprints/ST_DialogueOption Structure")) :!type "/Game/Blueprints/ST_Dialogue Structure"))
  (set `self.Starting Position` (`SceneComponent.K2_GetComponentLocation` (`self.CapsuleComponent`))))