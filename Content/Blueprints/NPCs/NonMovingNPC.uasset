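; NonMovingNPC is a stationary NPC that gives the player a short, dismissive dialogue exchange.
; It disables character movement on BeginPlay.
; The construction script fills the Dialogue array with one reply option tagged code 0.
; CodeTrigger handles the conversation by code: code 0 ends the dialogue, and any other code shows the NPC's rebuff with that option.
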(event `self.ReceiveBeginPlay`
  (`CharacterMovementComponent.DisableMovement` (`self.CharacterMovement`)))

(event `self.codeTrigger`
  (params (code :type Integer))
  (switch `int` code
    (:`Default`
      (`self.chooseDialogue` (`|GetArrayItem` (`self.dialogue`)) "Don't talk to me. Ever."))
    (:`0`
      (`self.endDialogue`))))

(fn `UserConstructionScript`
  (`parent.UserConstructionScript`)
  (set `self.dialogue` (`|MakeArray` (make `/Game/Blueprints/ST_Dialogue` (`|MakeArray` (make `/Game/Blueprints/ST_DialogueOption` "Yeah right ok, no problem, have a good-") :!type "/Game/Blueprints/ST_DialogueOption Structure")) :!type "/Game/Blueprints/ST_Dialogue Structure")))