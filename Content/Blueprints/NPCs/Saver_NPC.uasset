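; Saver NPC that runs a short dialogue asking the player to pray for forgiveness, then declares they won't be saved.
; The construction script fills a Dialogue array of response sets, pairing each line with a follow-up code.
; CodeTrigger switches on that code to open the prompt, show the rejection or end the conversation.
; Both opening responses share one code, so either choice gets the same rejection.
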(event `self.codeTrigger`
  (params (code :type Integer))
  (switch `int` code
    (:`Default`
      (`self.chooseDialogue` (`|GetArrayItem` (`self.dialogue`)) "PRAY FOR FORGIVENESS?"))
    (:`0`
      (`self.endDialogue`))
    (:`1`
      (`self.chooseDialogue` (`|GetArrayItem` (`self.dialogue`) 1) "YOU WON'T BE SAVED."))))

(fn `UserConstructionScript`
  (`parent.UserConstructionScript`)
  (set `self.dialogue` (`|MakeArray` (make `/Game/Blueprints/ST_Dialogue` (`|MakeArray` (make `/Game/Blueprints/ST_DialogueOption` "I would but uh, I don't believe in a higher power." 1) (make `/Game/Blueprints/ST_DialogueOption` "Yes" 1) :!type "/Game/Blueprints/ST_DialogueOption Structure")) (make `/Game/Blueprints/ST_Dialogue` (`|MakeArray` (make `/Game/Blueprints/ST_DialogueOption` "Dang, thanks though.") :!type "/Game/Blueprints/ST_DialogueOption Structure")) :!type "/Game/Blueprints/ST_Dialogue Structure")))