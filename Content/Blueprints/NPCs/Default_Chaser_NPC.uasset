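; Chaser NPC that runs at the player on sight to plead with them to take a flyer, using a short branching dialogue.
; Pawn sensing triggers a fast AI move to the player, then turns the player's camera toward the NPC on arrival.
; Being looked at starts dialogue, locks player movement and blocks further chases.
; Roaming resumes via delays, retriggered by repeat sightings, and both replies end the conversation.
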(event `self.whenLookedAt`
  (params (mainCharacter :type "/Game/Blueprints/BP_FP_Character Object Reference"))
  (bind _player_character (`self.Player Character`))
  (`self.lookAt` mainCharacter)
  (if (`KismetSystemLibrary.IsValid` (`self.Player Character`))
    (`KismetSystemLibrary.DelayUntilNextTick`)
    (`/Game/Blueprints/BP_FP_Character.startDialogue` _player_character)
    (`CharacterMovementComponent.DisableMovement` (`Character.CharacterMovement` _player_character))
    (set `self.convo` true)
    (set `self.Player Character` null)
    (`KismetSystemLibrary.Delay` 1.0)
    (`self.Random Roam`)))

(event `self.PawnSensing.OnSeePawn`
  (params (Pawn :type "Pawn Object Reference"))
  (if (not (or (`self.approaching`) (`self.convo`)))
    (bind _asbp_fp_character (cast `/Game/Blueprints/BP_FP_Character` Pawn))
    (set `self.Player Character` _asbp_fp_character)
    (`|ExecutionSequence`
      (:`then_0`
        (set `self.approaching` true)
        (set `CharacterMovementComponent.MaxWalkSpeed` 1000.0 (`self.CharacterMovement`))
        (`|AIMoveTo` self (0.0 0.0 0.0) (`self.Player Character`) 300.0
          (:`OnSuccess`
            (`Controller.SetControlRotation` (`GameplayStatics.GetPlayerController` 0) (`KismetMathLibrary.FindLookAtRotation` (`self.K2_GetActorLocation` (`self.Player Character`)) (- (`self.K2_GetActorLocation` self) (0.0 0.0 60.0)))))))
      (:`then_1`
        (`KismetSystemLibrary.RetriggerableDelay` 1.0 :!label _label)
        (`self.Random Roam`)))
    (else
      (goto _label))))

(event `self.codeTrigger`
  (params (code :type Integer))
  (switch `int` code
    (:`Default`
      (`self.chooseDialogue` (`|GetArrayItem` (`self.dialogue`)) "Please take this flyer please please please please please they have my family"))
    (:`0`
      (`self.endDialogue`))))

(fn `UserConstructionScript`
  (`parent.UserConstructionScript`)
  (set `self.dialogue` (`|MakeArray` (make `/Game/Blueprints/ST_Dialogue` (`|MakeArray` (make `/Game/Blueprints/ST_DialogueOption` "No.") (make `/Game/Blueprints/ST_DialogueOption` "Yeah totally. Thanks, I'll check this out!") :!type "/Game/Blueprints/ST_DialogueOption Structure")) :!type "/Game/Blueprints/ST_Dialogue Structure")))