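; BP_DialogueCharacter is an NPC character template for dialogue, with free-roam movement and placeholder hooks for dialogue setup.
; On BeginPlay, if Sense is unset or false, it walks to random reachable points around itself, picking a new one only after each successful move.
; The empty construction script is intended for defining dialogue options, and the empty codeTrigger event for switching on integer option codes.
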(event `self.ReceiveBeginPlay`
  ;[1 1 1] AI free roam
  (if (not (`self.sense`))
    (`self.Random Roam`)))

(event `Random Roam`
  ;[1 1 1] AI free roam
  (set `CharacterMovementComponent.MaxWalkSpeed` 200.0 (`self.CharacterMovement`))
  (`|AIMoveTo` self (`NavigationSystemV1.K2_GetRandomReachablePointInRadius` (`self.K2_GetActorLocation`) 2500.0 null null) null
    (:`OnSuccess`
      (`self.Random Roam`))))

(event `codeTrigger`
  (params (code :type Integer)))

(fn `UserConstructionScript`)