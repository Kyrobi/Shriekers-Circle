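; Dialogue NPC that offers help getting into the Law School and hands the player a red card key.
; The construction script defines two sets of replies, each tagged with a code that CodeTrigger switches on.
; Accepting spawns a RedCard_Pickup in front of the NPC, warns the player to run, then after a delay calls SpawnMonster and ends dialogue.
; Declining ends dialogue and calls ReturnToPost.
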(event `self.codeTrigger`
  (params (code :type Integer))
  (switch `int` code
    (:`Default`
      (`self.chooseDialogue` (`|GetArrayItem` (`self.dialogue`)) "Trying to get into the Law School?"))
    (:`0`
      (`self.endDialogue`)
      (`self.ReturnToPost`))
    (:`1`
      (`|SpawnActorFromClass` "/Game/Inventory/RedCard_Pickup.RedCard_Pickup_C" (`KismetMathLibrary.MakeTransform` (+ (* (`self.GetActorForwardVector`) 300) (`self.K2_GetActorLocation`))) "Undefined" "MultiplyWithRoot" null null)
      (`self.chooseDialogue` (`|GetArrayItem` (`self.dialogue`) 1) "Take this key and run!")
      (`KismetSystemLibrary.Delay` 5.0)
      (`self.SpawnMonster`)
      (`self.endDialogue`))))

(fn `UserConstructionScript`
  (`parent.UserConstructionScript`)
  (set `self.dialogue` (`|MakeArray` (make `/Game/Blueprints/ST_Dialogue` (`|MakeArray` (make `/Game/Blueprints/ST_DialogueOption` "Yeah, can you help?" 1) (make `/Game/Blueprints/ST_DialogueOption` "No.") :!type "/Game/Blueprints/ST_DialogueOption Structure")) (make `/Game/Blueprints/ST_Dialogue` (`|MakeArray` (make `/Game/Blueprints/ST_DialogueOption` "Ok.") (make `/Game/Blueprints/ST_DialogueOption` "Huh?") :!type "/Game/Blueprints/ST_DialogueOption Structure")) :!type "/Game/Blueprints/ST_Dialogue Structure")))