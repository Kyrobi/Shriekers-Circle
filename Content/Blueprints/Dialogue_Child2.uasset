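; Child character Blueprint that makes an AI chase pawns it sees, despite the dialogue-themed name.
; When PawnSensing spots a pawn, it sets a Sense flag, raises walk speed and moves toward that pawn.
; A retriggerable delay restarts on each sighting and calls RandomRoam, defined outside this file, about a second after the last one.
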(event `self.PawnSensing.OnSeePawn`
  (params (Pawn :type "Pawn Object Reference"))
  (set `self.sense` true)
  (`|ExecutionSequence`
    (:`then_0`
      (set `CharacterMovementComponent.MaxWalkSpeed` 1000.0 (`self.CharacterMovement`))
      (`|AIMoveTo` self (0.0 0.0 0.0) Pawn))
    (:`then_1`
      (`KismetSystemLibrary.RetriggerableDelay` 1.0)
      (`self.Random Roam`))))

(fn `UserConstructionScript`
  (`parent.UserConstructionScript`))