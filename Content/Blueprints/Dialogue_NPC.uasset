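; Example talking NPC that fills in a short dialogue set and reacts to the code of each line.
; The construction script builds the Dialogue array as one set of text and code pairs.
; CodeTrigger switches on the code to re-show that set while printing the name or jumping, or to end the dialogue.
; The re-show branches then reset Code to zero.
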(event `self.codeTrigger`
  (params (code :type Integer))
  (bind _output (`|GetArrayItem` (`self.dialogue`)))
  (switch `int` code
    (:`Default`
      (`self.chooseDialogue` _output)
      (`KismetSystemLibrary.PrintString` (`self.name`))
      (set `self.code` 0 :!label _label))
    (:`1`
      (`self.chooseDialogue` _output)
      (`self.Jump`)
      (goto _label))
    (:`2`
      (`self.endDialogue`))))

(fn `UserConstructionScript`
  (`parent.UserConstructionScript`)
  (set `self.dialogue` (`|MakeArray` (make `/Game/Blueprints/ST_Dialogue` (`|MakeArray` (make `/Game/Blueprints/ST_DialogueOption` "hi i'm the main character") (make `/Game/Blueprints/ST_DialogueOption` "can you jump?" 1) (make `/Game/Blueprints/ST_DialogueOption` "bye" 2) :!type "/Game/Blueprints/ST_DialogueOption Structure")) :!type "/Game/Blueprints/ST_Dialogue Structure")))