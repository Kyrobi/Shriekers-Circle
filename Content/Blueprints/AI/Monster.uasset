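; Monster AI pawn that wanders at random and chases pawns it sees.
; Shortly after spawning, it starts moving to random reachable points within a fixed radius, picking another after each successful move unless it had already sensed a pawn.
; PawnSensing sightings send it after the seen pawn, while a retriggerable delay resumes roaming once sightings stop for a second.
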(event `self.ReceiveBeginPlay`
  (`self.OnSpawn`))

(event `OnSpawn`
  ;[1 1 1] AI free roam
  (`KismetSystemLibrary.Delay` 1.5)
  (if (not (`self.sense`))
    (`self.Random Roam`)))

(event `Random Roam`
  ;[1 1 1] AI free roam
  (`|AIMoveTo` self (`NavigationSystemV1.K2_GetRandomReachablePointInRadius` (`self.K2_GetActorLocation`) 2500.0 null null) null
    (:`OnSuccess`
      (`self.Random Roam`))))

(event `self.PawnSensing.OnSeePawn`
  (params (Pawn :type "Pawn Object Reference"))
  (set `self.sense` true)
  (`|ExecutionSequence`
    (:`then_0`
      (`|AIMoveTo` self (0.0 0.0 0.0) Pawn))
    (:`then_1`
      (`KismetSystemLibrary.RetriggerableDelay` 1.0)
      (`self.Random Roam`))))

(fn `UserConstructionScript`)