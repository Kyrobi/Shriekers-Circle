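; First-person player character Blueprint that detects dialogue NPCs and runs conversations with them.
; Tick line-traces from the camera and, when the target changes outside menus, stores any BP_DialogueCharacter and shows or removes an interaction notification.
; Pressing E opens the dialogue widget created at BeginPlay and binds to the NPC's EndDialogue dispatcher to close it.
; Shared menu events toggle the cursor and menu flag, restoring game-only input on close.
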(event `menuClosed`
  (bind _returnvalue (`GameplayStatics.GetPlayerController` 0))
  ;[1 1 1] standard actions whenever a menu is closed
  (set `self.isMenuOpen` false)
  (set `PlayerController.bShowMouseCursor` false _returnvalue)
  (`WidgetBlueprintLibrary.SetInputMode_GameOnly` _returnvalue))

(event `menuOpened`
  ;[1 1 1] standard actions whenever a menu is opened
  (`Widget.RemoveFromParent` (`self.NotificationMenu`))
  (set `self.isMenuOpen` true)
  (set `PlayerController.bShowMouseCursor` true (`GameplayStatics.GetPlayerController` 0)))

(event `Key|E`
  (params (Key :type "Key Structure"))
  ;[1 1 1] opens dialogue with an NPC (if the NPC is valid)
  (:`Pressed`
    (if (`KismetSystemLibrary.IsValid` (`self.Dialogue Character`))
      (`self.startDialogue`))))

(event `self.ReceiveBeginPlay`
  ;[1 1 1] creates menus
  (bind _returnvalue (`|GenericCreateObject` "/Game/Blueprints/UI_DialogueMenu.UI_DialogueMenu_C"))
  (set `self.dialogueMenu` _returnvalue)
  (bind _returnvalue_2 (`|GenericCreateObject` "/Game/Blueprints/UI_InteractionNotification.UI_InteractionNotification_C"))
  (set `self.NotificationMenu` _returnvalue_2))

(event `self.ReceiveTick`
  (params (DeltaSeconds :type "Float (single-precision)"))
  (bind _firstpersoncamera (`self.FirstPersonCamera`))
  (bind _notificationmenu (`self.NotificationMenu`))
  (bind _returnvalue (`SceneComponent.K2_GetComponentLocation` _firstpersoncamera))
  ;[1 1 1] Scans objects the player looks at within 500 units
  (bind _outhit (`KismetSystemLibrary.LineTraceSingle` :`Start` _returnvalue :`End` (+ _returnvalue (* (`SceneComponent.GetForwardVector` _firstpersoncamera) 500.0)) :`TraceChannel` "TraceTypeQuery1" :`DrawDebugType` "ForOneFrame"))
  ;[1 1 1] updates 'viewTarget' only if there is a change and a menu is not open
  (if (and (!= (`self.viewTarget`) (`.HitActor` (`GameplayStatics.BreakHitResult` _outhit))) (not (`self.isMenuOpen`)))
    (bind _output_get (set `self.viewTarget` (`.HitActor` (`GameplayStatics.BreakHitResult` _outhit))))
    (bind _asbp_dialogue_character (cast `/Game/Blueprints/BP_DialogueCharacter` _output_get)
      (:`then`
        ;[1 1 1] stores reference to NPC and shows interaction message
        (set `self.Dialogue Character` _asbp_dialogue_character)
        (`/Game/Blueprints/UI_InteractionNotification.showMessage` _notificationmenu "NewEnumerator0"))
      (:`CastFailed`
        ;[1 1 1] unsets NPC reference and closes interaction message
        (set `self.Dialogue Character` null)
        (`Widget.RemoveFromParent` _notificationmenu)))))

(event `startDialogue`
  (`self.menuOpened`)
  (`UserWidget.AddToViewport` (`self.dialogueMenu`) 0)
  (`/Game/Blueprints/UI_DialogueMenu.startDialogue` (`self.dialogueMenu`) (`self.Dialogue Character`))
  ;[1 1 1] allows NPC to trigger 'endDialogue' event
  (add `/Game/Blueprints/BP_DialogueCharacter.endDialogue` (`self.Dialogue Character`) (`|CreateDelegate` :!event `endDialogue`)))

(event `endDialogue`
  (`self.menuClosed`)
  (`Widget.RemoveFromParent` (`self.dialogueMenu`))
  (clear `/Game/Blueprints/BP_DialogueCharacter.endDialogue` (`self.Dialogue Character`)))

(fn `UserConstructionScript`
  (`parent.UserConstructionScript`))